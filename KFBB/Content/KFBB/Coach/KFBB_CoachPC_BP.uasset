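; Player controller for the coach in KFBB, handling camera-style pawn movement, tile selection and debug spawning.
; Four axis inputs set directional velocities, which Tick sums to move the pawn without sweep.
; Mouse clicks forward touch, release and selection-clearing to inherited functions, while other inputs spawn players or a ball on tiles and Tab cycles tile debug state.
; Key 1 tries the GAS pickup-ball ability on the selected player and prints the result.
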(event `self.ReceiveBeginPlay`)

(event `Key|Tab`
  (params (Key :type "Key Structure"))
  (:`Pressed`
    (`self.NextTileDebugState`)))

(event `self.ReceiveTick`
  (params (DeltaSeconds :type "Float (single-precision)"))
  (bind _returnvalue (`self.K2_GetPawn`))
  (`self.K2_SetActorLocation` _returnvalue (+ (`self.K2_GetActorLocation` _returnvalue) (* (+ (`self.Move_Forward`) (`self.Move_Backward`) (`self.Move_Left`) (`self.Move_Right`)) DeltaSeconds)) false false))

(event `InputAction|RMB_Click`
  (params (Key :type "Key Structure"))
  (:`Pressed`
    (`self.ClearTileSelection` true)))

(event `InputAction|LMB_Click`
  (params (Key :type "Key Structure"))
  (:`Pressed`
    (`self.PlayerTouchScreen`))
  (:`Released`
    (`self.PlayerUntouchScreen`)))

(event `InputAxis|Axis_Forward`
  (params (AxisValue :type "Float (single-precision)"))
  (set `self.Move_Forward` (* (`self.Direction_Forward`) (* AxisValue (`self.Speed_Forward`)))))

(event `InputAction|SpawnPlayer`
  (params (Key :type "Key Structure"))
  (:`Pressed`
    (`self.SpawnPlayerOnTile` 0)))

(event `InputAction|SpawnBall`
  (params (Key :type "Key Structure"))
  (:`Pressed`
    (`self.SpawnBallOnTile`)))

(event `InputAction|SpawnOther`
  (params (Key :type "Key Structure"))
  (:`Pressed`
    (`self.SpawnPlayerOnTile` 1)))

(event `InputAxis|Axis_Backward`
  (params (AxisValue :type "Float (single-precision)"))
  (set `self.Move_Backward` (* (`self.Direction_Backward`) (* AxisValue (`self.Speed_Backward`)))))

(event `InputAxis|Axis_Left`
  (params (AxisValue :type "Float (single-precision)"))
  (set `self.Move_Left` (* (`self.Direction_Left`) (* AxisValue (`self.Speed_Left`)))))

(event `Key|One`
  (params (Key :type "Key Structure"))
  (:`Pressed`
    (bind _selectedplayer (`self.SelectedPlayer`)
      (:`then`
        (bind _returnvalue (`AbilitySystemComponent.TryActivateAbilityByClass` (`AbilitySystemBlueprintLibrary.GetAbilitySystemComponent` _selectedplayer) "/Game/KFBB/Player/Abilities/Pickup/GA_PickupBall.GA_PickupBall_C" true))
        (`KismetSystemLibrary.PrintString` (`KismetStringLibrary.Conv_BoolToString` _returnvalue)))
      (:`else`))))

(event `InputAxis|Axis_Right`
  (params (AxisValue :type "Float (single-precision)"))
  (set `self.Move_Right` (* (`self.Direction_Right`) (* AxisValue (`self.Speed_Right`)))))

(fn `UserConstructionScript`)